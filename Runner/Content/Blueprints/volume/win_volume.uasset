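; Level exit volume that completes the level when the player pawn overlaps its Win component with no crystals left.
; On overlap it searches for remaining BP_CYSTAL actors and prints a Polish prompt to collect the missing crystals if any exist.
; Otherwise it finds the current level in the LevelNames array and opens the next entry by name, or quits the game on the last one.
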(event OnComponentBeginOverlap(win)
  (params (OverlappedComponent :type Primitive%20Component%20Object%20Reference) (OtherActor :type Actor%20Object%20Reference) (OtherComp :type Primitive%20Component%20Object%20Reference) (OtherBodyIndex :type Integer) (bFromSweep :type Boolean) (SweepResult :type Hit%20Result%20Structure%20%28by%20ref%29))
  (if (== OtherActor (Game|Player|GetPlayerPawn 0))
    (bind _outactors (Actor|GetAllActorsOfClass "/Game/Blueprints/BP_CYSTAL.BP_CYSTAL_C"))
    (if (> (Utilities|Array|Length _outactors) 0)
      (Development|PrintString "Zbierz brakujące kryształy.")
      (else
        (level_manager|CompliteLevel)))))

(fn ConstructionScript)

(fn GetNextLevelName
  (return (Utilities|Array|Get(acopy) (Variables|Default|Getlevel_names) (+ (level_manager|GetCurentLevelIndex) 1))))

(fn IsFinalLevel
  (return (== (level_manager|GetCurentLevelIndex) (Utilities|Array|LastIndex (Variables|Default|Getlevel_names)))))

(fn LoadNewLevel
  (Game|OpenLevel(byName) (level_manager|GetNextLevelName)))

(fn CompliteLevel
  (if (level_manager|IsFinalLevel)
    (Game|QuitGame 0 "Quit" false)
    (else
      (level_manager|LoadNewLevel))))

(fn GetCurentLevelIndex
  (bind _returnvalue (Game|GetCurrentLevelName true))
  (return (Utilities|Array|FindItem (Variables|Default|Getlevel_names) (Utilities|String|StringToName _returnvalue))))