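; BP_CONE is an actor that gets drawn into the player and disappears on contact, like a pickup.
; When the player pawn overlaps its Trigger, a timeline lerps the actor's location toward the player and its scale toward zero, then destroys it.
; The timeline also sets Conelight intensity for an intended blink, but both lerp endpoints are zero, so the light is set to zero.
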(event OnComponentBeginOverlap(trigger)
  (params (OverlappedComponent :type Primitive%20Component%20Object%20Reference) (OtherActor :type Actor%20Object%20Reference) (OtherComp :type Primitive%20Component%20Object%20Reference) (OtherBodyIndex :type Integer) (bFromSweep :type Boolean) (SweepResult :type Hit%20Result%20Structure%20%28by%20ref%29))
  (if (== OtherActor (Game|Player|GetPlayerPawn 0))
    (bind (_direction _location _scale _light) (Timeline|Timeline_conechangelocation Play)
      (:Update
        ;[0.875 1 0.5573] przyciaganie
        (Transformation|SetActorLocation (Math|Vector|Lerp(Vector) (Transformation|GetActorLocation) (Transformation|GetActorLocation (Game|Player|GetPlayerPawn 0)) _location) false false)
        ;[0.8536 0.6114 1] zmniejszanie
        (Transformation|SetActorScale3D (Math|Vector|Lerp(Vector) (Transformation|GetActorScale3D) "0, 0, 0" _scale))
        ;[1 1 1] mruganie
        (Rendering|Components|Light|SetIntensity (Variables|Default|Getconelight) (Math|Float|Lerp 0.0 0.0 _light)))
      (:Finished
        (Actor|DestroyActor)))
    (else
      (Development|PrintString ""))))

(fn ConstructionScript)