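; BP_CYSTAL is a crystal actor that vanishes when the player pawn touches it, with no score or inventory change in its graphs.
; Overlap on the TRig component waits a brief delay, plays a 2D sound and starts a timeline.
; The timeline dims Crystallight and shrinks the actor, lerping from current values each update so the change compounds, then destroys the actor on finish.
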(event OnComponentBeginOverlap(TRig)
  (params (OverlappedComponent :type Primitive%20Component%20Object%20Reference) (OtherActor :type Actor%20Object%20Reference) (OtherComp :type Primitive%20Component%20Object%20Reference) (OtherBodyIndex :type Integer) (bFromSweep :type Boolean) (SweepResult :type Hit%20Result%20Structure%20%28by%20ref%29))
  (bind _crystallight (Variables|Default|Getcrystallight))
  (if (== OtherActor (Game|Player|GetPlayerPawn 0))
    (Utilities|FlowControl|Delay 0.07)
    (Audio|SpawnSound2D "/Game/Blueprints/S_CRYSTAL.S_CRYSTAL" 1.0 1.0 0.0 0)
    (bind (_direction _light _scale) (Timeline|Timeline_conechangelocation Play)
      (:Update
        ;[1 1 1] mruganie
        (Rendering|Components|Light|SetIntensity _crystallight (Math|Float|Lerp (Variables|/Script/Engine.LightComponentBase|GetIntensity _crystallight) 0.0 _light))
        ;[0.8536 0.6114 1] zmniejszanie
        (Transformation|SetActorScale3D (Math|Vector|Lerp(Vector) (Transformation|GetActorScale3D) "0, 0, 0" _scale)))
      (:Finished
        (Actor|DestroyActor)))))

(fn ConstructionScript)